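; BP_Star is an actor whose sphere material reacts to how close the first-person character is.
; On BeginPlay it finds the player character, creates a dynamic material instance on the sphere and sets its "proximity" parameter to 1.
; Each tick while the player overlaps the collision sphere, it sets proximity to their distance divided by the sphere's scaled radius.
; An older loop creating instances for every material is left disconnected.
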(event `self.ReceiveBeginPlay`
  (bind _sphere (`self.Sphere`))
  (`|ExecutionSequence`
    (:`then_0`
      (bind _returnvalue (`GameplayStatics.GetActorOfClass` "/Game/FirstPerson/Blueprints/BP_FirstPersonCharacter.BP_FirstPersonCharacter_C"))
      (set `self.firstPersonChar` _returnvalue))
    (:`then_1`
      (bind _returnvalue_2 (`PrimitiveComponent.CreateDynamicMaterialInstance` _sphere 0 (`PrimitiveComponent.GetMaterial` _sphere 0) "None"))
      (set `self.DMI` _returnvalue_2))
    (:`then_2`
      (`MaterialInstanceDynamic.SetScalarParameterValue` (`self.DMI`) "proximity" 1.0))))

(event `self.ReceiveTick`
  (params (DeltaSeconds :type "Float (single-precision)"))
  (if (`PrimitiveComponent.IsOverlappingActor` (`self.SphereCol`) (`self.firstPersonChar`))
    (`MaterialInstanceDynamic.SetScalarParameterValue` (`self.DMI`) "proximity" (/ (`self.GetDistanceTo` (`self.firstPersonChar`)) (`SphereComponent.GetScaledSphereRadius` (`self.SphereCol`))))))

(fn `UserConstructionScript`)