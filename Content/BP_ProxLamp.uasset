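; BP_ProxLamp is a lamp that brightens as the first-person character approaches and changes color when looked at.
; BeginPlay caches the character, turns the light off and creates a dynamic material for the sphere.
; While the character overlaps SphereCol, Tick maps distance over radius to light intensity and the material's proximity parameter.
; A camera-forward dot product threshold picks between two colors for both light and material.
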(event `self.ReceiveBeginPlay`
  (bind _sphere (`self.Sphere`))
  (`|ExecutionSequence`
    (:`then_0`
      (bind _returnvalue (`GameplayStatics.GetActorOfClass` "/Game/FirstPerson/Blueprints/BP_FirstPersonCharacter.BP_FirstPersonCharacter_C"))
      (set `self.firstPersonChar` _returnvalue)
      (`LightComponent.SetIntensity` (`self.PointLight`) 0.0))
    (:`then_1`
      (bind _returnvalue_2 (`PrimitiveComponent.CreateDynamicMaterialInstance` _sphere 0 (`PrimitiveComponent.GetMaterial` _sphere 0) "None"))
      (set `self.DMI` _returnvalue_2))
    (:`then_2`
      (`MaterialInstanceDynamic.SetScalarParameterValue` (`self.DMI`) "proximity" 1.0))))

(event `self.ReceiveTick`
  (params (DeltaSeconds :type "Float (single-precision)"))
  (bind _color1 (`self.color1`))
  (bind _color2 (`self.color2`))
  (bind _returnvalue (/ (`self.GetDistanceTo` (`self.firstPersonChar`)) (`SphereComponent.GetScaledSphereRadius` (`self.SphereCol`))))
  (if (`PrimitiveComponent.IsOverlappingActor` (`self.SphereCol`) (`self.firstPersonChar`))
    (set `self.distRadiusRatio` _returnvalue)
    (`LightComponent.SetIntensity` (`self.PointLight`) (* 3000.0 (- 1.0 _returnvalue)))
    (`MaterialInstanceDynamic.SetScalarParameterValue` (`self.DMI`) "proximity" (`self.distRadiusRatio`))
    (if (> (`KismetMathLibrary.Dot_VectorVector` (`KismetMathLibrary.Normal` (- (`self.K2_GetActorLocation`) (`SceneComponent.K2_GetComponentLocation` (`/Game/FirstPerson/Blueprints/BP_FirstPersonCharacter.FirstPersonCamera` (`self.firstPersonChar`))))) (`SceneComponent.GetForwardVector` (`/Game/FirstPerson/Blueprints/BP_FirstPersonCharacter.FirstPersonCamera` (`self.firstPersonChar`)))) 0.9)
      (`MaterialInstanceDynamic.SetVectorParameterValue` (`self.DMI`) "color" _color1)
      (`LightComponent.SetLightColor` (`self.PointLight`) _color1 true)
      (else
        (`MaterialInstanceDynamic.SetVectorParameterValue` (`self.DMI`) "color" _color2)
        (`LightComponent.SetLightColor` (`self.PointLight`) _color2 true)))))

(fn `UserConstructionScript`)